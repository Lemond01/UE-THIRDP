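; BP_Monster is an enemy that damages the player on contact with its HazardZone.
; At BeginPlay it sets its damage to half the player's current health, read by casting player pawn 0 to BP_ThirdPersonCharacter.
; An overlap by a Player-tagged actor damages that pawn and clears CanAttack.
; The attack re-arms one second after an overlap ends, so staying inside the zone causes no repeat hits.
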(event `self.HazardZone.OnComponentEndOverlap`
  (params (OverlappedComponent :type "PrimitiveComponent Object Reference") (OtherActor :type "Actor Object Reference") (OtherComp :type "PrimitiveComponent Object Reference") (OtherBodyIndex :type Integer))
  (if (not (`self.CanAttack`))
    (`KismetSystemLibrary.Delay` 1.0)
    (set `self.CanAttack` true)))

(event `self.HazardZone.OnComponentBeginOverlap`
  (params (OverlappedComponent :type "PrimitiveComponent Object Reference") (OtherActor :type "Actor Object Reference") (OtherComp :type "PrimitiveComponent Object Reference") (OtherBodyIndex :type Integer) (bFromSweep :type Boolean) (SweepResult :type "HitResult Structure (by ref)"))
  (if (`self.ActorHasTag` OtherActor "Player")
    (if (`self.CanAttack`)
      (bind (_playerhealth _target) (`self.GetPlayerCurrentHealth`))
      (`GameplayStatics.ApplyDamage` _target (stale `self.ReceiveBeginPlay` _output_get_2))
      (set `self.CanAttack` false))))

(event `self.ReceiveBeginPlay`
  (bind _playerhealth (`self.GetPlayerCurrentHealth`))
  (bind _output_get (set `self.PlayerHealth` _playerhealth))
  (bind _output_get_2 (set `self.Damage` (/ _output_get 2.0))))

(fn `GetPlayerCurrentHealth`
  (returns (PlayerHealth :type "Float (double-precision)") (Target :type "/Game/ThirdPerson/Blueprints/BP_ThirdPersonCharacter Object Reference"))
  (bind _asbp_third_person_character (cast `/Game/ThirdPerson/Blueprints/BP_ThirdPersonCharacter` (`GameplayStatics.GetPlayerPawn` 0)))
  (return (`/Game/ThirdPerson/Blueprints/BP_ThirdPersonCharacter.Health` _asbp_third_person_character) _asbp_third_person_character))

(fn `UserConstructionScript`)