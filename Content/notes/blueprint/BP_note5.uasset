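; BP_note5 is an interactable note actor that the player can read and put away.
; Its Interaction event uses a FlipFlop: the first call creates the WB_notas widget, hides the Nota component and ignores the player's look and move input.
; The next call invokes the widget's DropDawn, shows the note again and restores input, with a paper sound played on both toggles.
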(event `self.interaction`
  (bind _returnvalue (`GameplayStatics.GetPlayerController` 0))
  (bind _nota (`self.nota`))
  (bind _returnvalue_2 (`SceneComponent.K2_GetComponentLocation` (`self.nota`)))
  (`/Engine/EditorBlueprintResources/StandardMacros.FlipFlop`
    (:`A`
      (`GameplayStatics.PlaySoundAtLocation` "/Game/notes/sonido/papel.papel" _returnvalue_2 (struct) 1.0 1.0 0.0 null null null null)
      (bind _returnvalue_3 (`|CreateWidget` "/Game/notes/widgets/WB_notas.WB_notas_C"))
      (`UserWidget.AddToViewport` _returnvalue_3 0)
      (`Controller.SetIgnoreLookInput` _returnvalue true)
      (`Controller.SetIgnoreMoveInput` _returnvalue true)
      (`SceneComponent.SetVisibility` _nota false false))
    (:`B`
      (`GameplayStatics.PlaySoundAtLocation` "/Game/notes/sonido/papel.papel" _returnvalue_2 (struct) 1.0 1.0 0.0 null null null null)
      (`/Game/notes/widgets/WB_notas.DropDawn` _returnvalue_3)
      (`Controller.SetIgnoreLookInput` _returnvalue false)
      (`Controller.SetIgnoreMoveInput` _returnvalue false)
      (`SceneComponent.SetVisibility` _nota true false))))

(fn `UserConstructionScript`)