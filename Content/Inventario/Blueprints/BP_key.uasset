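; BP_key is an inventory-related Blueprint that checks whether the player holds the key for a door.
; Its TengoLlave function loops through the Inventario array and compares each entry's Quantity with the Quantity on the BPDoor reference, rather than a key ID.
; On a match it sets HasKey on the character reference and prints a debug message.
; The event graph holds only disabled default events, and nothing in this file calls TengoLlave.
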(fn `tengoLlave`
  (for _array_element (`self.inventario`)
    (if (== (`/Game/Inventario/Blueprints/BP_Door.quantity` (`self.BPDoor`)) (`.Quantity_8_46BF799E4D28CFB96A5912B659D9097D` (break `/Game/Inventario/Blueprints/S_ItemStucture` _array_element)))
      (set `/Game/ThirdPerson/Blueprints/BP_ThirdPersonCharacter.hasKey` true (`self.bpcharacter`))
      (`KismetSystemLibrary.PrintString` "player has the key"))))

(fn `UserConstructionScript`
  (`parent.UserConstructionScript`))